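; BP_SceneController is a player input actor that, judging by its calls, relates to a rhythm controller.
; It enables input on BeginPlay and pairs W, S, A and D with the top, bottom, left and right gamepad face buttons.
; Each pair shares a press path that only calls GetPlayerRhythmController, with nothing done with the result yet.
; Tick, overlap and construction logic are empty.
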(event `self.ReceiveBeginPlay`
  (`self.EnableInput` null))

(event `Key|SpaceBar`
  (params (Key :type "Key Structure")))

(event `Key|W`
  (params (Key :type "Key Structure"))
  (:`Pressed`
    (`self.GetPlayerRhythmController` :!label _label)))

(event `Key|Gamepad_FaceButton_Top`
  (params (Key :type "Key Structure"))
  (:`Pressed`
    (goto _label)))

(event `Key|S`
  (params (Key :type "Key Structure"))
  (:`Pressed`
    (`self.GetPlayerRhythmController` :!label _label_2)))

(event `Key|Gamepad_FaceButton_Bottom`
  (params (Key :type "Key Structure"))
  (:`Pressed`
    (goto _label_2)))

(event `Key|A`
  (params (Key :type "Key Structure"))
  (:`Pressed`
    (`self.GetPlayerRhythmController` :!label _label_3)))

(event `Key|Gamepad_FaceButton_Left`
  (params (Key :type "Key Structure"))
  (:`Pressed`
    (goto _label_3)))

(event `Key|D`
  (params (Key :type "Key Structure"))
  (:`Pressed`
    (`self.GetPlayerRhythmController` :!label _label_4)))

(event `Key|Gamepad_FaceButton_Right`
  (params (Key :type "Key Structure"))
  (:`Pressed`
    (goto _label_4)))

(fn `UserConstructionScript`)