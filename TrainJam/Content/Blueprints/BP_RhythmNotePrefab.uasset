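; BP_RhythmNotePrefab is an arrow note actor for a rhythm game, shown on a Plane component.
; Its Spawningarrow event reads the arrow type and switches on the direction to give the plane a colored material and rotate the actor to match.
; It then calls SetArrowPos, which, like GetArrowType, is defined outside this graph.
; BeginPlay, Tick, overlap and the construction script do nothing.
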(event `self.Spawningarrow`
  (bind _plane (`self.Plane`))
  (bind _returnvalue (`self.GetArrowType`))
  (switch `string` _returnvalue
    (:`Up`
      (`PrimitiveComponent.SetMaterial` _plane 0 "/Game/Materials/Rhythm/GreenArrow.GreenArrow")
      (`self.K2_SetActorRotation` (struct :`Yaw` -90.0 :`Roll` -90.0)))
    (:`Down`
      (`PrimitiveComponent.SetMaterial` _plane 0 "/Game/Materials/Rhythm/BlueArrow.BlueArrow")
      (`self.K2_SetActorRotation` (struct :`Yaw` 90.0 :`Roll` 90.0)))
    (:`Left`
      (`PrimitiveComponent.SetMaterial` _plane 0 "/Game/Materials/Rhythm/YellowArrow.YellowArrow")
      (`self.K2_SetActorRotation` (struct :`Pitch` -90.0 :`Roll` 180.0)))
    (:`Right`
      (`PrimitiveComponent.SetMaterial` _plane 0 "/Game/Materials/Rhythm/RedArrow.RedArrow")
      (`self.K2_SetActorRotation` (struct :`Pitch` 90.0))))
  (`self.SetArrowPos`))

(fn `UserConstructionScript`)