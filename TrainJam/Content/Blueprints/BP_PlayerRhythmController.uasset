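; BP_PlayerRhythmController is the player's hit marker for a rhythm game, checking directional input against arrow notes.
; On each input event, it recolors Cube1 with a material matching the pressed direction.
; It then scans every BP_RhythmNotePrefab actor and destroys those with a matching arrow type within a narrow window of Cube1 along the Y axis.
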(event `self.InputEvent`
  (bind _cube1 (`self.Cube1`))
  (bind (_returnvalue_x _returnvalue_y) (`KismetMathLibrary.BreakVector` (`SceneComponent.K2_GetComponentLocation` (`self.Cube1`))))
  (bind _returnvalue (`self.GetInputType`))
  (switch `string` _returnvalue
    (:`Up`
      (`PrimitiveComponent.SetMaterial` _cube1 0 "/Game/Materials/Colors/Green.Green"))
    (:`Down`
      (`PrimitiveComponent.SetMaterial` _cube1 0 "/Game/Materials/Colors/Blue.Blue"))
    (:`Left`
      (`PrimitiveComponent.SetMaterial` _cube1 0 "/Game/Materials/Colors/Yellow.Yellow"))
    (:`Right`
      (`PrimitiveComponent.SetMaterial` _cube1 0 "/Game/Materials/Colors/Red.Red")))
  (bind _outactors (`GameplayStatics.GetAllActorsOfClass` "/Game/Blueprints/BP_RhythmNotePrefab.BP_RhythmNotePrefab_C"))
  (for _array_element _outactors
    (bind _returnvalue_2 (`RhythmNoteScript.GetArrowType` _array_element))
    (if (`KismetStringLibrary.EqualEqual_StrStr` _returnvalue _returnvalue_2)
      (bind (_returnvalue_x_2 _returnvalue_y_2) (`KismetMathLibrary.BreakVector` (`SceneComponent.K2_GetComponentLocation` (`Actor.RootComponent` _array_element))))
      (bind _returnvalue_3 (- _returnvalue_y_2 _returnvalue_y))
      (if (< _returnvalue_3 50.0)
        (if (> _returnvalue_3 -50.0)
          (`self.K2_DestroyActor` _array_element))))))

(fn `UserConstructionScript`)